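; Player character Blueprint that handles movement, jumping, taking damage and losing the game.
; Axis inputs move it along the control rotation's forward and right vectors, and the Jump press triggers a jump.
; Any damage briefly swaps a body material as a hit flash, then subtracts from Health and prints it.
; At zero or less Health, it casts to BP_MyGameMode and calls GameResult with false.
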(event Custom|DamagedBody
  (Rendering|Material|SetMaterial (Variables|Character|GetMesh) 2 "/Game/Materials/T_Liz_Body_Mat_2.T_Liz_Body_Mat_2")
  (Utilities|FlowControl|Delay 0.2)
  (Rendering|Material|SetMaterial (Variables|Character|GetMesh) 2 "/Game/Materials/T_Liz_Body_Mat.T_Liz_Body_Mat"))

(event Custom|GameOver
  (bind _asbp_my_game_mode (Utilities|Casting|CastToBP_MyGameMode (Game|GetGameMode)))
  (Default|GameResult _asbp_my_game_mode false))

(event EventBeginPlay)

(event Collision|EventActorBeginOverlap
  (params (OtherActor :type Actor%20Object%20Reference)))

(event EventTick
  (params (DeltaSeconds :type Float%20%28single-precision%29)))

(event Game|Damage|EventAnyDamage
  (params (Damage :type Float%20%28single-precision%29) (DamageType :type Damage%20Type%20Object%20Reference) (InstigatedBy :type Controller%20Object%20Reference) (DamageCauser :type Actor%20Object%20Reference))
  (CallFunction|DamagedBody)
  (bind _output_get (Variables|Default|SetHealth (- (Variables|Default|GetHealth) Damage)))
  (Development|PrintString (Utilities|String|ToString(Float) _output_get))
  (if (<= _output_get 0.0)
    (CallFunction|GameOver)))

(event Input|ActionEvents|InputActionJump
  (params (Key :type Key%20Structure :default "None"))
  (:Pressed
    (Character|Jump)))

(event Input|AxisEvents|InputAxisMoveForward
  (params (AxisValue :type Float%20%28single-precision%29))
  (Pawn|Input|AddMovementInput (Math|Vector|GetForwardVector (Pawn|GetControlRotation :!class /Script/Engine.Pawn)) AxisValue false))

(event Input|AxisEvents|InputAxisMoveRight
  (params (AxisValue :type Float%20%28single-precision%29))
  (Pawn|Input|AddMovementInput (Math|Vector|GetRightVector (Pawn|GetControlRotation :!class /Script/Engine.Pawn)) AxisValue false))

(fn ConstructionScript)